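; BP_Planks is a collectible plank pickup that the first-person player gathers with the pickup input.
; A box overlap with the first-person character enables and disables the actor's input, so pickup only works nearby.
; Picking up decrements the game mode's Remaining count, shows a collected widget, and destroys the plank.
; The last plank's widget also shows shore instructions, while earlier ones hide the instruction text.
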(event `EnhancedInput|/Game/Input/Actions/IA_Pickup`
  (params (ActionValue :type Boolean) (ElapsedSeconds :type "Float (double-precision)") (TriggeredSeconds :type "Float (double-precision)") (InputAction :type "InputAction Object Reference" :default "/Game/Input/Actions/IA_Pickup.IA_Pickup"))
  (:`Started`
    (bind _asbp_first_person_game_mode (cast `/Game/FirstPerson/Blueprints/BP_FirstPersonGameMode` (`GameplayStatics.GetGameMode`)))
    (bind _result (`/Engine/EditorBlueprintResources/StandardMacros.DecrementInt` (`/Game/FirstPerson/Blueprints/BP_FirstPersonGameMode.Remaining` _asbp_first_person_game_mode))
      (:`  `
        (set `/Game/FirstPerson/Blueprints/BP_FirstPersonGameMode.Remaining` _result _asbp_first_person_game_mode)
        (if (== (`/Game/FirstPerson/Blueprints/BP_FirstPersonGameMode.Remaining` _asbp_first_person_game_mode) 0)
          (bind _returnvalue (`|CreateWidget` "/Game/Blueprints/WB_Collected.WB_Collected_C"))
          (`/Game/Blueprints/WB_Collected.ShowShoreInstructions` _returnvalue)
          (`UserWidget.AddToViewport` _returnvalue 0)
          (else
            (bind _returnvalue_2 (`|CreateWidget` "/Game/Blueprints/WB_Collected.WB_Collected_C"))
            (`Widget.SetVisibility` (`/Game/Blueprints/WB_Collected.InstructionText` _returnvalue_2) "Hidden")
            (`UserWidget.AddToViewport` _returnvalue_2 0)))
        (`self.K2_DestroyActor`)))))

(event `self.Box.OnComponentBeginOverlap`
  (params (OverlappedComponent :type "PrimitiveComponent Object Reference") (OtherActor :type "Actor Object Reference") (OtherComp :type "PrimitiveComponent Object Reference") (OtherBodyIndex :type Integer) (bFromSweep :type Boolean) (SweepResult :type "HitResult Structure (by ref)"))
  (cast `/Game/FirstPerson/Blueprints/BP_FirstPersonCharacter` OtherActor)
  (`self.EnableInput` (`GameplayStatics.GetPlayerController` 0)))

(event `self.Box.OnComponentEndOverlap`
  (params (OverlappedComponent :type "PrimitiveComponent Object Reference") (OtherActor :type "Actor Object Reference") (OtherComp :type "PrimitiveComponent Object Reference") (OtherBodyIndex :type Integer))
  (cast `/Game/FirstPerson/Blueprints/BP_FirstPersonCharacter` OtherActor)
  (`self.DisableInput` (`GameplayStatics.GetPlayerController` 0)))

(fn `UserConstructionScript`)